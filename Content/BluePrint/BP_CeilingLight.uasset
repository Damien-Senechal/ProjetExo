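; BP_CeilingLight is a ceiling light actor that turns on while another actor overlaps it.
; The construction script sets the starting color, and BeginPlay switches the light off after a short delay.
; Begin overlap applies the variable intensity, then changes to a second color after a delay.
; End overlap sets intensity to zero but leaves the color unchanged.
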(event EventBeginPlay
  (Utilities|FlowControl|Delay 1.0)
  (Rendering|Components|Light|SetIntensity (Variables|Default|GetPointLight) 0.0))

(event Collision|EventActorBeginOverlap
  (params (OtherActor :type Actor%20Object%20Reference))
  (Rendering|Components|Light|SetIntensity (Variables|Default|GetPointLight) (Variables|Default|GetIntensity_%20Variable))
  (Utilities|FlowControl|Delay 1.0)
  (Rendering|Components|Light|SetLightColor (Variables|Default|GetPointLight) (Variables|Default|GetNew%20Light%20Color) false))

(event Collision|EventActorEndOverlap
  (params (OtherActor :type Actor%20Object%20Reference))
  (Rendering|Components|Light|SetIntensity (Variables|Default|GetPointLight) 0.0))

(fn ConstructionScript
  (Rendering|Components|Light|SetLightColor (Variables|Default|GetPointLight) (Variables|Default|GetStarting%20Light%20Color) true))